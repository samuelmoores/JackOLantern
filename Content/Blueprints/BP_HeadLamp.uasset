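; BP_HeadLamp is a head lamp pickup that the player character can wear as a light.
; Until picked up, its mesh yaws a fixed step each Tick with the spotlight at zero intensity.
; Interact attaches it to the third-person character's head socket, turns the spotlight on and sets PickedUp, after which Tick zeroes the mesh's relative rotation.
; The player-tag overlap check leads to no action.
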(event EventBeginPlay
  (Rendering|Components|Light|SetIntensity (Variables|Default|GetSpotLight) 0.0))

(event Collision|EventActorBeginOverlap
  (params (OtherActor :type Actor%20Object%20Reference))
  (if (Actor|ActorHasTag OtherActor "Player")
    _))

(event EventTick
  (params (DeltaSeconds :type Float%20%28single-precision%29))
  (bind _mesh (Variables|Default|GetMesh))
  (bind _returnvalue (Transformation|GetWorldRotation _mesh))
  (if (not (Variables|Default|GetpickedUp))
    (Transformation|SetWorldRotation _mesh (Math|Rotator|MakeRotator (.roll _returnvalue) (.pitch _returnvalue) (+ (.yaw _returnvalue) 1.0)) false false)
    (else
      (Transformation|SetRelativeRotation _mesh "0, 0, 0" false false))))

(event EventInteract
  (Transformation|SetWorldRotation (Variables|Default|GetMesh) "0, 0, 0" false false)
  (bind _asbp_third_person_character (Utilities|Casting|CastToBP_ThirdPersonCharacter (Game|GetPlayerCharacter 0)))
  (Transformation|AttachComponentToComponent (Variables|/Script/Engine.Character|GetMesh _asbp_third_person_character) "head_SOC" "SnapToTarget" "KeepRelative" "SnapToTarget" true)
  (Rendering|Components|Light|SetIntensity (Variables|Default|GetSpotLight) 5e+03)
  (Variables|Default|SetpickedUp true))

(fn ConstructionScript)