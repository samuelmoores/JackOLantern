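; BP_Door is a key-locked door that opens when the player interacts while holding a matching key.
; Interact casts the player character to BP_ThirdPersonCharacter and loops through its Keys array for an actor tagged with the door's third tag.
; On the first match it calls Open, plays the DoorOpening sound in 2D and stops searching; without a match nothing happens.
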(event EventBeginPlay)

(event Collision|EventActorBeginOverlap
  (params (OtherActor :type Actor%20Object%20Reference)))

(event EventTick
  (params (DeltaSeconds :type Float%20%28single-precision%29)))

(event EventInteract
  (bind _asbp_third_person_character (Utilities|Casting|CastToBP_ThirdPersonCharacter (Game|GetPlayerCharacter 0)))
  (bind _array_element (Utilities|Array|ForEachLoopwithBreak (Variables|/Game/ThirdPerson/Blueprints/BP_ThirdPersonCharacter.BP_ThirdPersonCharacter_C|GetKeys _asbp_third_person_character) :!label _label)
    (:LoopBody
      (if (Actor|ActorHasTag _array_element (Utilities|Array|Get(acopy) (Variables|Default|GetTags self) 2))
        (Class|Door|Open)
        (Audio|PlaySound2D "/Game/Audio/Door-Opening.Door-Opening" 1.0 1.0 0.0 0 0)
        (goto _label Break)))))

(fn ConstructionScript)