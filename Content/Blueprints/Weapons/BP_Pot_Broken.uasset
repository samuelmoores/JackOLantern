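; Broken pot actor whose mesh shards settle under physics, then reassemble into their spawn arrangement.
; BeginPlay plays a reverse-shatter sound, caches each shard's world transform and starts a timeline.
; Once the timeline passes one second and the first shard's velocity is zero, it disables physics and records the scattered transforms.
; Timeline updates then lerp all shards back using an alpha accumulated from delta seconds, rewinding the break.
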(event EventBeginPlay
  (Audio|PlaySound2D "/Game/Audio/Shattering_Reverse.Shattering_Reverse" 1.0 1.0 0.0 0 0)
  (Utilities|Array|Add (Variables|Default|Getmeshes) (Variables|Default|GetSM_Pot_Broken_polySurface37))
  (Utilities|Array|Add (Variables|Default|Getmeshes) (Variables|Default|GetSM_Pot_Broken_polySurface38))
  (Utilities|Array|Add (Variables|Default|Getmeshes) (Variables|Default|GetSM_Pot_Broken_polySurface39))
  (Utilities|Array|Add (Variables|Default|Getmeshes) (Variables|Default|GetSM_Pot_Broken_polySurface40))
  (Utilities|Array|Add (Variables|Default|Getmeshes) (Variables|Default|GetSM_Pot_Broken_polySurface41))
  (Utilities|Array|Add (Variables|Default|Getmeshes) (Variables|Default|GetSM_Pot_Broken_polySurface42))
  (Utilities|Array|Add (Variables|Default|Getmeshes) (Variables|Default|GetSM_Pot_Broken_polySurface43))
  (Utilities|Array|Add (Variables|Default|Getmeshes) (Variables|Default|GetSM_Pot_Broken_polySurface44))
  (Utilities|Array|Add (Variables|Default|Getmeshes) (Variables|Default|GetSM_Pot_Broken_polySurface45))
  (Utilities|Array|Add (Variables|Default|Getmeshes) (Variables|Default|GetSM_Pot_Broken_polySurface46))
  (Utilities|Array|Add (Variables|Default|Getmeshes) (Variables|Default|GetSM_Pot_Broken_polySurface47))
  (Utilities|Array|Add (Variables|Default|Getmeshes) (Variables|Default|GetSM_Pot_Broken_polySurface48))
  (Utilities|Array|Add (Variables|Default|Getmeshes) (Variables|Default|GetSM_Pot_Broken_polySurface49))
  (Utilities|Array|Add (Variables|Default|Getmeshes) (Variables|Default|GetSM_Pot_Broken_polySurface50))
  (Utilities|Array|Add (Variables|Default|Getmeshes) (Variables|Default|GetSM_Pot_Broken_polySurface51))
  (Utilities|Array|Add (Variables|Default|Getmeshes) (Variables|Default|GetSM_Pot_Broken_polySurface52))
  (Utilities|Array|Add (Variables|Default|Getmeshes) (Variables|Default|GetSM_Pot_Broken_polySurface53))
  (Utilities|Array|Add (Variables|Default|Getmeshes) (Variables|Default|GetSM_Pot_Broken_polySurface54))
  (Utilities|Array|Add (Variables|Default|Getmeshes) (Variables|Default|GetSM_Pot_Broken_polySurface55))
  (Utilities|Array|Add (Variables|Default|Getmeshes) (Variables|Default|GetSM_Pot_Broken_polySurface56))
  (Utilities|Array|Add (Variables|Default|Getmeshes) (Variables|Default|GetSM_Pot_Broken_polySurface57))
  (Utilities|Array|Add (Variables|Default|Getmeshes) (Variables|Default|GetSM_Pot_Broken_polySurface58))
  (Utilities|Array|Add (Variables|Default|Getmeshes) (Variables|Default|GetSM_Pot_Broken_polySurface59))
  (for _array_element (Variables|Default|Getmeshes)
    (Utilities|Array|Add (Variables|Default|GetspawnLocations) (Transformation|GetWorldLocation _array_element))
    (Utilities|Array|Add (Variables|Default|GetspawnRotations) (Transformation|GetWorldRotation _array_element)))
  (bind _time (Timeline|Timeline Play)
    (:Update
      (Variables|Default|SetTime _time)
      (if (and (> _time 1.0) (<= (Math|Vector|VectorLength (Transformation|GetComponentVelocity (Variables|Default|GetSM_Pot_Broken_polySurface37))) 0.0))
        (Utilities|FlowControl|Sequence
          (:then_0
            (Utilities|FlowControl|DoOnce false
              (:Completed
                (for _array_element_2 (Variables|Default|Getmeshes)
                  (Physics|SetSimulatePhysics _array_element_2 false)
                  (Utilities|Array|Add (Variables|Default|GetfinishedShatterLocations) (Transformation|GetWorldLocation _array_element_2))
                  (Utilities|Array|Add (Variables|Default|GetfinishedShatterRotations) (Transformation|GetWorldRotation _array_element_2))))))
          (:then_1
            (bind _output_get (Variables|Default|SetAlpha (+ (Utilities|Time|GetWorldDeltaSeconds) (Variables|Default|GetAlpha))))
            (for (_array_element_3 _array_index) (Variables|Default|Getmeshes)
              (Transformation|SetWorldLocation _array_element_3 (Math|Vector|Lerp(Vector) (Utilities|Array|Get(acopy) (Variables|Default|GetfinishedShatterLocations) _array_index) (Utilities|Array|Get(acopy) (Variables|Default|GetspawnLocations) _array_index) (Math|Float|Clamp(Float) _output_get)) false false)
              (Transformation|SetWorldRotation _array_element_3 (Math|Rotator|Lerp(Rotator) (Utilities|Array|Get(acopy) (Variables|Default|GetfinishedShatterRotations) _array_index) (Utilities|Array|Get(acopy) (Variables|Default|GetspawnRotations) _array_index) (Math|Float|Clamp(Float) _output_get)) false false))))))))

(fn ConstructionScript)