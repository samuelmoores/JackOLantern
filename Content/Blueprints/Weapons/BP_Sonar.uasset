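; BP_Sonar is a weapon actor that damages the player when it hits them while its Moving flag is set.
; On Hit it prints the struck component's name, then checks for the Player tag and Moving.
; A valid hit applies damage only if the BP_ThirdPersonCharacter's Damaged flag is clear, then sets that flag to block repeat damage.
; Any hit that fails the tag or movement check clears Moving.
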(event EventBeginPlay)

(event EventTick
  (params (DeltaSeconds :type Float%20%28single-precision%29)))

(event Collision|EventHit
  (params (MyComp :type Primitive%20Component%20Object%20Reference) (Other :type Actor%20Object%20Reference) (OtherComp :type Primitive%20Component%20Object%20Reference) (bSelfMoved :type Boolean) (HitLocation :type Vector :default "0, 0, 0") (HitNormal :type Vector :default "0, 0, 0") (NormalImpulse :type Vector :default "0, 0, 0") (Hit :type Hit%20Result%20Structure%20%28by%20ref%29))
  (Development|PrintString (Utilities|GetDisplayName OtherComp))
  (if (and (Actor|ActorHasTag Other "Player") (Variables|Default|Getmoving))
    (bind _asbp_third_person_character (Utilities|Casting|CastToBP_ThirdPersonCharacter Other))
    (if (not (Variables|/Script/Project_JackOLantern.Project_JackOLanternCharacter|Getdamaged _asbp_third_person_character))
      (Game|Damage|ApplyDamage _asbp_third_person_character 0.0 0 0)
      (Variables|/Script/Project_JackOLantern.Project_JackOLanternCharacter|Setdamaged _asbp_third_person_character true))
    (else
      (Variables|Default|Setmoving false))))

(event Collision|EventActorBeginOverlap
  (params (OtherActor :type Actor%20Object%20Reference)))

(fn ConstructionScript)