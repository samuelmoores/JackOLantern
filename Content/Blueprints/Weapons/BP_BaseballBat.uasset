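; Baseball bat weapon that the player picks up, carries and can damage enemies with.
; Interact attaches it to the player's hand socket once, then sets the character's bat flag and weapon state and updates the HUD.
; ChangeWeapon, marked as a weapon interface event, moves it between back and right-hand sockets based on weapon state.
; Overlap caches Enemy-tagged actors as the target for DoDamage, which is not called within this Blueprint.
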(event EventChangeWeapon
  (bind _player (Variables|Default|GetPlayer))
  ;[1 1 1] Toggle between hand and back sockets - Weapon Interface
  (Utilities|IsValid _player
    (:Is%20Valid
      (if (Variables|/Script/Project_JackOLantern.Project_JackOLanternCharacter|GethasBat _player)
        (switch Utilities|FlowControl|Switch|SwitchonWeaponState (Class|ProjectJackOLanternCharacter|GetJackStateWeapon (Variables|Default|GetPlayer))
          (:UNARMED
            (Variables|Default|SetSocket%20Name "spine04_Socket"))
          (:HAS_BAT
            (Variables|Default|SetSocket%20Name "hand_r_Socket")))
        (Transformation|AttachComponentToComponent (Variables|/Script/Engine.Character|GetMesh (Variables|Default|GetPlayer)) (Variables|Default|GetSocket%20Name) "SnapToTarget" "SnapToTarget" "KeepRelative" true)))))

(event EventInteract
  (bind _returnvalue (Game|GetPlayerCharacter 0))
  ;[1 1 1] Player Pickup - Interact Interface
  (Utilities|IsValid _returnvalue
    (:Is%20Valid
      (bind _asbp_third_person_character (Utilities|Casting|CastToBP_ThirdPersonCharacter _returnvalue))
      (Variables|Default|SetPlayer _asbp_third_person_character)
      (Variables|Default|SetpickedUp true)
      (Utilities|FlowControl|DoOnce false
        (:Completed
          (bind _returnvalue_2 (Transformation|AttachComponentToComponent (Variables|/Script/Engine.Character|GetMesh (Variables|Default|GetPlayer)) "hand_l_SOC" "SnapToTarget" "SnapToTarget" "KeepRelative" true))
          (Variables|/Script/Project_JackOLantern.Project_JackOLanternCharacter|SethasBat (Variables|Default|GetPlayer) _returnvalue_2)
          ;[1 1 1] ENUM for animation
          (Class|ProjectJackOLanternCharacter|SetWeaponState (Variables|Default|GetPlayer) "HAS_BAT")
          ;[1 1 1] Update HUD
          (Default|ChangeWeapon (Variables|/Game/ThirdPerson/Blueprints/BP_ThirdPersonCharacter.BP_ThirdPersonCharacter_C|GetHUD (Variables|Default|GetPlayer))))))))

(event Collision|EventActorBeginOverlap
  (params (OtherActor :type Actor%20Object%20Reference))
  (bind _returnvalue (Actor|ActorHasTag OtherActor "Enemy"))
  ;[1 1 1] Has bat overlapped an enemy? - if yes, get ref
  (Variables|Default|SetenemyOverlapped _returnvalue)
  (if _returnvalue
    (bind _asenemy (Utilities|Casting|CastToEnemy OtherActor))
    (Variables|Default|SetEnemy _asenemy)))

(fn ConstructionScript)

(fn DoDamage
  (Game|Damage|ApplyDamage (Variables|Default|GetEnemy) 1.0 0 0))