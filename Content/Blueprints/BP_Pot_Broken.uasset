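; Broken pot actor made of shard meshes that settle, drift back toward their starting arrangement and are then removed.
; BeginPlay records each shard's world transform and starts a fast looping timer that waits for one reference shard to stop moving.
; The timer then disables physics on all shards and gradually lerps them toward the saved transforms using delta seconds.
; During this phase, it destroys the actor once Lifetime has elapsed since spawn.
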(event Custom|Spawn
  (bind _returnvalue (Utilities|Time|SetTimerbyFunctionName 0 "RunDestroyTimer" 0.01 true))
  (Variables|Default|SetTimer _returnvalue))

(event Custom|Destroy
  (Actor|DestroyActor))

(event EventBeginPlay
  (Variables|Default|SettimeOfSpawn (Utilities|Time|GetTimeSeconds))
  (Utilities|Array|Add (Variables|Default|Getmeshes) (Variables|Default|GetSM_Pot_Broken_polySurface48))
  (Utilities|Array|Add (Variables|Default|Getmeshes) (Variables|Default|GetSM_Pot_Broken_polySurface44))
  (Utilities|Array|Add (Variables|Default|Getmeshes) (Variables|Default|GetSM_Pot_Broken_polySurface45))
  (Utilities|Array|Add (Variables|Default|Getmeshes) (Variables|Default|GetSM_Pot_Broken_polySurface46))
  (Utilities|Array|Add (Variables|Default|Getmeshes) (Variables|Default|GetSM_Pot_Broken_polySurface47))
  (Utilities|Array|Add (Variables|Default|Getmeshes) (Variables|Default|GetSM_Pot_Broken_polySurface37))
  (Utilities|Array|Add (Variables|Default|Getmeshes) (Variables|Default|GetSM_Pot_Broken_polySurface38))
  (Utilities|Array|Add (Variables|Default|Getmeshes) (Variables|Default|GetSM_Pot_Broken_polySurface39))
  (Utilities|Array|Add (Variables|Default|Getmeshes) (Variables|Default|GetSM_Pot_Broken_polySurface42))
  (Utilities|Array|Add (Variables|Default|Getmeshes) (Variables|Default|GetSM_Pot_Broken_polySurface40))
  (Utilities|Array|Add (Variables|Default|Getmeshes) (Variables|Default|GetSM_Pot_Broken_polySurface54))
  (Utilities|Array|Add (Variables|Default|Getmeshes) (Variables|Default|GetSM_Pot_Broken_polySurface41))
  (Utilities|Array|Add (Variables|Default|Getmeshes) (Variables|Default|GetSM_Pot_Broken_polySurface43))
  (Utilities|Array|Add (Variables|Default|Getmeshes) (Variables|Default|GetSM_Pot_Broken_polySurface56))
  (Utilities|Array|Add (Variables|Default|Getmeshes) (Variables|Default|GetSM_Pot_Broken_polySurface57))
  (Utilities|Array|Add (Variables|Default|Getmeshes) (Variables|Default|GetSM_Pot_Broken_polySurface55))
  (Utilities|Array|Add (Variables|Default|Getmeshes) (Variables|Default|GetSM_Pot_Broken_polySurface58))
  (Utilities|Array|Add (Variables|Default|Getmeshes) (Variables|Default|GetSM_Pot_Broken_polySurface59))
  (Utilities|Array|Add (Variables|Default|Getmeshes) (Variables|Default|GetSM_Pot_Broken_polySurface50))
  (Utilities|Array|Add (Variables|Default|Getmeshes) (Variables|Default|GetSM_Pot_Broken_polySurface51))
  (Utilities|Array|Add (Variables|Default|Getmeshes) (Variables|Default|GetSM_Pot_Broken_polySurface49))
  (Utilities|Array|Add (Variables|Default|Getmeshes) (Variables|Default|GetSM_Pot_Broken_polySurface52))
  (Utilities|Array|Add (Variables|Default|Getmeshes) (Variables|Default|GetSM_Pot_Broken_polySurface53))
  (for _array_element (Variables|Default|Getmeshes)
    (Utilities|Array|Add (Variables|Default|GetspawnLocations) (Transformation|GetWorldLocation _array_element))
    (Utilities|Array|Add (Variables|Default|GetspawnRotations) (Transformation|GetWorldRotation _array_element)))
  (CallFunction|Spawn))

(fn ConstructionScript)

(fn RunDestroyTimer
  (bind _returnvalue (Utilities|Time|GetWorldDeltaSeconds))
  (if (not (Variables|Default|Getspawned))
    (Variables|Default|Setspawned true)
    (else
      ;[1 1 1] Wait for it to stop moving
      (if (<= (Math|Vector|VectorLength (Transformation|GetComponentVelocity (Variables|Default|GetSM_Pot_Broken_polySurface43))) 0.0)
        ;[1 1 1] When did it stop moving?
        (if (Variables|Default|Getmoving)
          (Variables|Default|Setmoving false)
          (else
            (for (_array_element _array_index) (Variables|Default|Getmeshes)
              (Physics|SetSimulatePhysics _array_element false)
              (Transformation|SetWorldRotation _array_element (Math|Rotator|Lerp(Rotator) (Transformation|GetWorldRotation _array_element) (Utilities|Array|Get(acopy) (Variables|Default|GetspawnRotations) _array_index) _returnvalue) false false)
              (Transformation|SetWorldLocation _array_element (Math|Vector|Lerp(Vector) (Transformation|GetWorldLocation _array_element) (Utilities|Array|Get(acopy) (Variables|Default|GetspawnLocations) _array_index) _returnvalue) false false))
            (if (>= (- (Utilities|Time|GetTimeSeconds) (Variables|Default|GettimeOfSpawn)) (Variables|Default|GetLifetime))
              (CallFunction|Destroy))))))))