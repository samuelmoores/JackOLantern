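; Tableware cover that lifts open once when the player interacts with it.
; The first Interact captures the mesh's relative transform and computes an offset, raised position with added pitch.
; The Uncover timeline then lerps the location and drives the rotation through RInterpTo, feeding the track value in as delta time so it acts as a blend alpha.
; DoOnce is never reset, so the cover stays open.
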(event EventInteract
  (bind _mesh (Variables|Default|GetMesh))
  ;[1 1 1] Open on Interact
  (Utilities|FlowControl|DoOnce false
    (:Completed
      (bind _output_get (Variables|Default|SetstartLocation (Variables|/Script/Engine.SceneComponent|GetRelativeLocation _mesh)))
      (Variables|Default|SetendLocation (+ _output_get "-25.000000,0.000000,25.000000"))
      (bind _output_get_2 (Variables|Default|SetstartRotation (Variables|/Script/Engine.SceneComponent|GetRelativeRotation _mesh)))
      (Variables|Default|SetendRotation (Math|Rotator|MakeRotator (.roll _output_get_2) (+ (.pitch _output_get_2) 45.0) (.yaw _output_get_2)))
      (bind _newtrack_0 (Timeline|Uncover Play)
        (:Update
          (Transformation|SetRelativeLocation (Variables|Default|GetMesh) (Math|Vector|Lerp(Vector) (Variables|Default|GetstartLocation) (Variables|Default|GetendLocation) _newtrack_0) false false)
          (Transformation|SetRelativeRotation (Variables|Default|GetMesh) (Math|Interpolation|RInterpTo (Variables|Default|GetstartRotation) (Variables|Default|GetendRotation) _newtrack_0 1.0) false false))))))

(fn ConstructionScript)