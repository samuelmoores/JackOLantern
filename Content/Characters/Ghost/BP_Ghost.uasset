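; BP_Ghost is a ghost that periodically launches a BP_Sonar projectile while the player is nearby.
; It caches the third-person player character on BeginPlay and retries on Tick whenever that reference is invalid.
; Within range, a DoOnce gate spawns the sonar slightly above the ghost, impulses its mesh along that mesh's Z axis, then resets after a delay.
; The inline comments about knife, range and interval do not match the logic.
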(event EventBeginPlay
  (bind _asbp_third_person_character (Utilities|Casting|CastToBP_ThirdPersonCharacter (Game|GetPlayerCharacter 0)))
  (Variables|Default|SetPlayer _asbp_third_person_character))

(event EventTick
  (params (DeltaSeconds :type Float%20%28single-precision%29))
  (bind _returnvalue (Transformation|GetActorTransform))
  (Utilities|IsValid (Variables|Default|GetPlayer)
    (:Is%20Valid
      (if (< (Math|Vector|Distance(Vector) (Transformation|GetActorLocation (Variables|Default|GetPlayer)) (Transformation|GetActorLocation)) 1.35e+03)
        ;[1 1 1] spawn a knife slitly above the ghost
        (Utilities|FlowControl|DoOnce false :!label _label
          (:Completed
            (bind _returnvalue_2 (Game|SpawnActorfromClass "/Game/Blueprints/Weapons/BP_Sonar.BP_Sonar_C" (Math|Transform|MakeTransform (Math|Vector|MakeVector (.x (.location _returnvalue)) (.y (.location _returnvalue)) (+ (.z (.location _returnvalue)) 25.0)) (.rotation _returnvalue) (.scale _returnvalue)) "Undefined" "MultiplyWithRoot" 0 0))
            ;[1 1 1] launch the knife along the knives Z axis every 3 seconds
            (Physics|AddImpulse (Variables|/Game/Blueprints/Weapons/BP_Sonar.BP_Sonar_C|GetMesh _returnvalue_2) (* (.Z (Math|Rotator|GetAxes (Transformation|GetWorldRotation (Variables|/Game/Blueprints/Weapons/BP_Sonar.BP_Sonar_C|GetMesh _returnvalue_2)))) 1e+04) "None" false)
            (Utilities|FlowControl|Delay 1e+01)
            (goto _label Reset)))))
    (:Is%20Not%20Valid
      (bind _asbp_third_person_character (Utilities|Casting|CastToBP_ThirdPersonCharacter (Game|GetPlayerCharacter 0)))
      (Variables|Default|SetPlayer _asbp_third_person_character))))

(fn ConstructionScript)