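; BP_Pot_Broken is the broken version of the pot, an actor that removes itself once its Lifetime has elapsed.
; On BeginPlay it calls Spawn, which starts a fast looping timer, and records the spawn time.
; The timer runs RunDestroyTimer, which polls elapsed game time against Lifetime and calls Destroy to destroy the actor.
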(event Custom|Spawn
  (bind _returnvalue (Utilities|Time|SetTimerbyFunctionName 0 "RunDestroyTimer" 0.01 true))
  (Variables|Default|SetTimer _returnvalue))

(event Custom|Destroy
  (Actor|DestroyActor))

(event EventBeginPlay
  (CallFunction|Spawn)
  (Variables|Default|SettimeOfSpawn (Utilities|Time|GetTimeSeconds)))

(fn ConstructionScript)

(fn RunDestroyTimer
  (if (>= (- (Utilities|Time|GetTimeSeconds) (Variables|Default|GettimeOfSpawn)) (Variables|Default|GetLifetime))
    (CallFunction|Destroy)))