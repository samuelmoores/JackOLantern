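; AI controller for the zombie guard that runs the BT_Zombie behavior tree when it possesses a BP_Zombie_Guard.
; It caches the player character at BeginPlay and the guard pawn on possession.
; Every AI perception update writes its actor to the "Player" blackboard key, without filtering by class or whether it was sensed or lost.
; An unfinished check of the player's UnderTable state is left disconnected.
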(event OnTargetPerceptionUpdated(AIPerception)
  (params (Actor :type Actor%20Object%20Reference) (Stimulus :type AI%20Stimulus%20Structure))
  (AI|Components|Blackboard|SetValueasObject (Variables|Default|GetBlackboard) (Utilities|Name|MakeLiteralName "Player") Actor))

(event EventBeginPlay
  (bind _asbp_third_person_character (Utilities|Casting|CastToBP_ThirdPersonCharacter (Game|GetPlayerCharacter 0)))
  (Variables|Default|SetPlayer _asbp_third_person_character))

(event EventPossess
  (params (PossessedPawn :type Pawn%20Object%20Reference))
  (bind _asbp_zombie_guard (Utilities|Casting|CastToBP_Zombie_Guard PossessedPawn))
  (Variables|Default|SetZombie%20Guard _asbp_zombie_guard)
  (AI|RunBehaviorTree "/Game/Characters/Zombie/AI/BT_Zombie.BT_Zombie"))

(fn ConstructionScript)