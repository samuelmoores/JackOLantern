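; BP_Zombie is a zombie character Blueprint that carries a damage box and plays attack and death sounds.
; BeginPlay snaps the DamageBox to the pelvis socket, keeping its relative scale.
; Tick polls the Attacking and Dead flags, using DoOnce gates to play a moan once per attack and a choking sound once on death.
; Both sounds are non-spatial 2D, and neither flag is set in these graphs.
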(event EventBeginPlay
  (Transformation|AttachComponentToComponent (Variables|Default|GetDamageBox) 0 "pelvis" "SnapToTarget" "SnapToTarget" "KeepRelative" true))

(event EventTick
  (params (DeltaSeconds :type Float%20%28single-precision%29))
  (Utilities|FlowControl|Sequence
    (:then_0
      (if (Variables|Default|Getattacking)
        (Utilities|FlowControl|DoOnce false :!label _label
          (:Completed
            (Audio|PlaySound2D "/Game/Audio/Zombie-Moan.Zombie-Moan" 1.0 1.0 0.0 0 0)))
        (else
          (goto _label Reset))))
    (:then_1
      (if (Variables|Default|Getdead)
        (Utilities|FlowControl|DoOnce false
          (:Completed
            (Audio|PlaySound2D "/Game/Audio/Zombie-Dying-and-Choking.Zombie-Dying-and-Choking" 1.0 1.0 0.0 0 0)))))))

(fn ConstructionScript)